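; A collectable pickup actor that takes on a random item from DT_Collectables when Type is "none".
; The construction script applies the row's mesh, score and rarity overlay material, scaling the trigger sphere from mesh bounds plus CollectionRadius.
; Any overlap passes the row to player 0's BPC_Inventory, without checking the overlapping actor.
; The pickup then destroys itself unless that inventory reports full after collection.
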(event `self.ReceiveBeginPlay`)

(event `self.ReceiveActorBeginOverlap`
  (params (OtherActor :type "Actor Object Reference"))
  (bind _returnvalue (`self.GetComponentByClass` (`GameplayStatics.GetPlayerCharacter` 0) "/Game/ThirdPerson/Blueprints/BPC_Inventory.BPC_Inventory_C"))
  (`/Game/ThirdPerson/Blueprints/BPC_Inventory.CollectItem` _returnvalue (`self.Out Row`))
  (if (not (`/Game/ThirdPerson/Blueprints/BPC_Inventory.InventoryIsFull` _returnvalue))
    (`self.K2_DestroyActor`)))

(fn `UserConstructionScript`
  (bind _scaledistance (`self.ScaleDistance`))
  (bind _type (`self.Type`))
  (bind (_out_row_name _out_row_mesh _out_row_score _out_row_rarity) (break `/Game/Collectables/Strut_Collectables` (`self.Out Row`)))
  (bind _returnvalue (+ (/ (`.SphereRadius` (`KismetSystemLibrary.GetComponentBounds` (`self.CollectableBody`))) 40.0) (`self.CollectionRadius`)))
  (if (== _type "none")
    (bind _outrownames (`DataTableFunctionLibrary.GetDataTableRowNames` "/Game/Collectables/DT_Collectables.DT_Collectables"))
    (else
      (`KismetSystemLibrary.PrintString` (`KismetStringLibrary.Conv_NameToString` _type))))
  (bind _returnvalue_2 (`|GetDataTableRow` "/Game/Collectables/DT_Collectables.DT_Collectables" (`KismetArrayLibrary.Array_Random` _outrownames))
    (:`then`
      (bind _output_get (set `self.Out Row` _returnvalue_2))
      (set `self.CollectableScore` (`.Score_23_E0762692444023A61F2569A76C4A2319` (break `/Game/Collectables/Strut_Collectables` _output_get)))
      (bind _returnvalue_3 (`StaticMeshComponent.SetStaticMesh` (`self.CollectableBody`) (`.Mesh_20_361D7EE7411889E2AEE061A079D3B00E` (break `/Game/Collectables/Strut_Collectables` _output_get))))
      (`KismetMathLibrary.Vector_Set` _scaledistance _returnvalue _returnvalue _returnvalue)
      (if _returnvalue_3
        (`SceneComponent.SetRelativeScale3D` (`self.Sphere`) _scaledistance)
        (`MeshComponent.SetOverlayMaterial` (`self.CollectableBody`) _out_row_rarity)))))