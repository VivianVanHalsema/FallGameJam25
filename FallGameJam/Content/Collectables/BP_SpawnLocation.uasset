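; BP_SpawnLocation is a spawn point that places a random collectable in the world.
; Its CanBegin event waits briefly, then checks the CanSpawn flag, which this graph never sets.
; If the flag is true, it spawns a BP_CollectableObject at its root transform, passing a random PossibleItems entry as the Type.
; Otherwise it prints a debug message and destroys itself.
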(event `CanBegin`
  (`KismetSystemLibrary.Delay` 0.2)
  (if (`self.CanSpawn`)
    (bind _output_get (set `self.NewVar` (`KismetArrayLibrary.Array_Random` (`self.PossibleItems`))))
    (`|SpawnActorFromClass` "/Game/Collectables/BP_CollectableObject.BP_CollectableObject_C" (`SceneComponent.K2_GetComponentToWorld` (`self.DefaultSceneRoot`)) "Undefined" "MultiplyWithRoot" null _output_get null)
    (else
      (`KismetSystemLibrary.PrintString` "oh I die actually")
      (`self.K2_DestroyActor`))))

(fn `UserConstructionScript`)