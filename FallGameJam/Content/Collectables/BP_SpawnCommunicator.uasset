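; Spawn coordinator that, in its construction script, assigns rarity-based collectable pools to shuffled BP_SpawnLocation actors and starts each via CanBegin.
; It sorts DT_Collectables names into rarity arrays by outline material, then picks pools using random rolls and caps derived from ItemSpawnMax.
; As written, special pools require counts already at cap, the rare branch assigns UncommonArray, and CurrentItemSpawn never increments.
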(event `self.ReceiveBeginPlay`)

(fn `UserConstructionScript`
  (bind _currentspawnlocation (`self.CurrentSpawnLocation`))
  (bind _returnvalue (/ (`self.ItemSpawnMax`) 3))
  (bind _outrownames (`DataTableFunctionLibrary.GetDataTableRowNames` "/Game/Collectables/DT_Collectables.DT_Collectables"))
  (for _array_element _outrownames
    (bind _returnvalue_2 (`|GetDataTableRow` "/Game/Collectables/DT_Collectables.DT_Collectables" _array_element)
      (:`then`
        (if (== (`.Rarity_32_C455D700454B189BC71F428DC9349EC6` (break `/Game/Collectables/Strut_Collectables` _returnvalue_2)) "/Game/VFX/VFXMaterials/M_Outline_Common.M_Outline_Common")
          (`KismetArrayLibrary.Array_Add` (`self.CommonArray`) (break `/Game/Collectables/Strut_Collectables` _returnvalue_2))
          (elif (== (`.Rarity_32_C455D700454B189BC71F428DC9349EC6` (break `/Game/Collectables/Strut_Collectables` _returnvalue_2)) "/Game/VFX/VFXMaterials/M_Outline_Uncommon.M_Outline_Uncommon")
            (`KismetArrayLibrary.Array_Add` (`self.UncommonArray`) (break `/Game/Collectables/Strut_Collectables` _returnvalue_2))
            (elif (== (`.Rarity_32_C455D700454B189BC71F428DC9349EC6` (break `/Game/Collectables/Strut_Collectables` _returnvalue_2)) "/Game/VFX/VFXMaterials/M_Outline_Rare.M_Outline_Rare")
              (`KismetArrayLibrary.Array_Add` (`self.RareArray`) (break `/Game/Collectables/Strut_Collectables` _returnvalue_2))
              (else
                (`KismetArrayLibrary.Array_Add` (`self.LegendaryArray`) (break `/Game/Collectables/Strut_Collectables` _returnvalue_2)))))))))
  (set `self.CommonCap` (+ _returnvalue _returnvalue))
  (set `self.RareCap` (/ (`self.ItemSpawnMax`) 5))
  (set `self.LegendaryCap` (/ (`self.ItemSpawnMax`) 10))
  (bind _outactors (`GameplayStatics.GetAllActorsOfClass` "/Game/Collectables/BP_SpawnLocation.BP_SpawnLocation_C"))
  (`KismetArrayLibrary.Array_Shuffle` _outactors)
  (for _array_element_2 _outactors
    (if (<= (`self.CurrentItemSpawn`) (`self.ItemSpawnMax`))
      (bind _output_get (set `self.CurrentSpawnLocation` _array_element_2))
      (set `/Game/Collectables/BP_SpawnLocation.CanSpawn` true _output_get)
      (bind _output_get_2 (set `self.RandomItemChance` (`KismetMathLibrary.RandomIntegerInRange` 0 100)))
      (if (>= _output_get_2 90)
        (if (>= (`self.currLegendary`) (`self.LegendaryCap`))
          (set `/Game/Collectables/BP_SpawnLocation.PossibleItems` (`self.LegendaryArray`) (`self.CurrentSpawnLocation`))
          (set `self.currLegendary` (+ (`self.currLegendary`) 1))
          (else
            (if (>= _output_get_2 65) :!label _label
              (if (>= (`self.currRare`) (`self.RareCap`))
                (set `/Game/Collectables/BP_SpawnLocation.PossibleItems` (`self.UncommonArray`) (`self.CurrentSpawnLocation`))
                (set `self.currRare` (+ (`self.currRare`) 1))
                (else
                  (if (>= _output_get_2 20) :!label _label_2
                    (if (>= (`self.currCommon`) (`self.CommonCap`))
                      (set `/Game/Collectables/BP_SpawnLocation.PossibleItems` (`self.CommonArray`) _currentspawnlocation)
                      (set `self.currCommon` (+ (`self.currCommon`) 1))
                      (else
                        (set `/Game/Collectables/BP_SpawnLocation.PossibleItems` (`self.UncommonArray`) _currentspawnlocation :!label _label_3)))
                    (else
                      (goto _label_3)))))
              (else
                (goto _label_2)))))
        (else
          (goto _label)))
      (`/Game/Collectables/BP_SpawnLocation.CanBegin` _currentspawnlocation)
      (else
        (break)))))